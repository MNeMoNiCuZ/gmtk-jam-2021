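; Player character for a physics puzzle game where the player drags, lifts and rotates pieces, then moves between levels.
; Mouse traces pick DragComponent actors, which a PhysicsHandle moves within clamped bounds; the wheel sets lift and WASD rotates via tagged helper actors.
; Right-drag orbits a smoothed camera rig.
; When PuzzleManager reports all solved, pieces freeze, the camera spins and a timer triggers a post-process transition to the next level.
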(event AllSolved(PuzzleManager)
  (bind _hudmanager (Variables|Default|GetHUDManager))
  (Utilities|FlowControl|DoOnce false
    (:Completed
      (Components|Timeline|SetPlayRate (Variables|Default|GetTL_CompleteCameraCoolness) 1.0)
      (Audio|PlaySound2D "/Game/Sound/Stingers/Complete.Complete" 1.0 1.0 0.0 0 0)
      (Variables|Default|SetSolved true)
      (Utilities|FlowControl|Sequence
        (:then_0
          (bind _outactors (Actor|GetAllActorsOfClass "/Game/Pieces/BP_Piece_Base.BP_Piece_Base_C"))
          (for _array_element _outactors
            (Physics|SetSimulatePhysics (Variables|/Game/Pieces/BP_Piece_Base.BP_Piece_Base_C|GetSM_TestPiece_01 _array_element) false))
          (Default|RemoveHUDControls _hudmanager)
          (Default|AddHUDLevelComplete _hudmanager))
        (:then_1
          (bind _returnvalue (Utilities|Time|SetTimerbyEvent (delegate Custom|GoToNextLevel) 2e+01))
          (Variables|Default|SetNextLevelTimer _returnvalue))))))

(event Custom|InitiateTargetLerp
  (params (Source :type Vector))
  (bind _physicshandleworldlocation (Variables|Default|GetPhysicsHandleWorldLocation))
  (bind _physicsoffset (Variables|Default|GetPhysicsOffset))
  (bind _returnvalue (+ _physicshandleworldlocation _physicsoffset))
  (Variables|Default|SetTargetLerpActive true)
  (Variables|Default|SetSource Source)
  (bind (_direction _z _x_y) (Timeline|Tl_TargetLerp PlayFromStart)
    (:Update
      (Variables|Default|SetTargetLerp (Math|Vector|MakeVector (Math|Float|Lerp (.x (Variables|Default|GetSource)) (.x _returnvalue) _x_y) (Math|Float|Lerp (.y (Variables|Default|GetSource)) (.y _returnvalue) _x_y) (Math|Float|Lerp (.z (Variables|Default|GetSource)) (.z _returnvalue) _z))))
    (:Finished
      (Variables|Default|SetTargetLerpActive false))))

(event Custom|SetOverlap
  (params (OverlapActor :type Actor%20Object%20Reference))
  (Variables|Default|SetOverlap%20Actor OverlapActor))

(event Custom|EventPause
  (bind _hudmanager (Variables|Default|GetHUDManager))
  (Utilities|FlowControl|FlipFlop
    (:A
      (Default|AddHUDPause _hudmanager))
    (:B
      (Default|RemoveHUDPause _hudmanager))))

(event Custom|SetHeld
  (params (Held%20Actor :type Actor%20Object%20Reference))
  (bind _output_get (Variables|Default|SetHeld%20Actor Held%20Actor))
  (Utilities|IsValid _output_get
    (:Is%20Valid
      (bind _asprimitive_component (Utilities|Casting|CastToPrimitiveComponent (Variables|/Script/Engine.Actor|GetRootComponent _output_get)))
      (Variables|Default|SetPhysicsOffset (Math|Vector|MakeVector (.x (- (Transformation|GetActorLocation _output_get) (Variables|Default|GetPhysicsHandleWorldLocation))) (.y (- (Transformation|GetActorLocation _output_get) (Variables|Default|GetPhysicsHandleWorldLocation))) (+ (.z (- (Transformation|GetActorLocation _output_get) (Variables|Default|GetPhysicsHandleWorldLocation))) 2e+01)))
      (Physics|Components|PhysicsHandle|GrabComponentatLocationwithRotation (Variables|Default|GetPhysicsHandle) _asprimitive_component "None" (Transformation|GetActorLocation _output_get) "0, 0, 0")
      (CallFunction|InitiateTargetLerp (Transformation|GetActorLocation _output_get))
      (Transformation|SetActorRelativeRotation (Variables|Default|GetLol))
      (Variables|Default|SetLift 0.0))
    (:Is%20Not%20Valid
      (Physics|Components|PhysicsHandle|ReleaseComponent (Variables|Default|GetPhysicsHandle))
      (Variables|Default|SetPhysicsOffset "0, 0, 0")
      (Transformation|SetActorRotation (Variables|Default|GetReferenceRotation))
      (Transformation|SetActorRotation (Variables|Default|GetLol)))))

(event Custom|Update
  (params (AddRelativeRotation :type Rotator))
  (Transformation|AttachActorToActor (Variables|Default|GetReferenceRotation) (Variables|Default|GetLol) "None" "KeepWorld" "KeepWorld" "KeepWorld" true)
  (Transformation|SetActorRelativeRotation (Variables|Default|GetLol) AddRelativeRotation)
  (Transformation|DetachFromActor (Variables|Default|GetReferenceRotation) "KeepWorld" "KeepWorld" "KeepWorld")
  (Transformation|SetActorRelativeRotation (Variables|Default|GetLol))
  (Class|PhysicsHandleComponent|SetTargetRotation (Variables|Default|GetPhysicsHandle) (Transformation|GetActorRotation (Variables|Default|GetReferenceRotation))))

(event Custom|Reverse%20Camera
  (bind _nextlevel (Variables|Default|GetNextLevel))
  (Components|Timeline|SetPlayRate (Variables|Default|GetTL_CompleteCameraCoolness) 1.4)
  (Utilities|FlowControl|Delay 1.9)
  (Utilities|FlowControl|Sequence
    (:then_0
      (Audio|PlaySound2D "/Game/Sound/Stingers/NewLevel.NewLevel" 1.0 1.0 0.0 0 0)
      (bind (_direction _fov _vignetteramp) (Timeline|TL_CompleteCameraCoolness ReverseFromEnd)
        (:Update
          (Utilities|Struct|SetmembersinPostProcessSettings (Variables|/Script/Engine.PostProcessVolume|GetSettings (Variables|Default|GetPostVolume)) (Math|Vector4|MakeVector4 1.0 1.0 1.0 1.0) _vignetteramp))
        (:Finished
          (if (Utilities|Enum|Equal(Enum) _direction "Forward")
            (switch Utilities|FlowControl|Switch|SwitchonENUM_NextOrPreviousLevel (Variables|Default|GetNextOrPreviousLevel)
              (:NewEnumerator0
                (Default|GotoNextLevel _nextlevel))
              (:NewEnumerator1
                (Default|GotoPreviousLevel _nextlevel)))))))
    (:then_1
      (Utilities|FlowControl|Delay 1.0)
      (Default|AddHUDControls (Variables|Default|GetHUDManager)))))

(event Custom|TriggerCompleteCamera
  (bind _nextlevel (Variables|Default|GetNextLevel))
  (Audio|PlaySound2D "/Game/Sound/Stingers/ChangeLevel.ChangeLevel" 1.0 1.0 0.0 0 0)
  (bind (_direction _fov _vignetteramp) (Timeline|TL_CompleteCameraCoolness PlayFromStart)
    (:Update
      (Utilities|Struct|SetmembersinPostProcessSettings (Variables|/Script/Engine.PostProcessVolume|GetSettings (Variables|Default|GetPostVolume)) (Math|Vector4|MakeVector4 1.0 1.0 1.0 1.0) _vignetteramp))
    (:Finished
      (if (Utilities|Enum|Equal(Enum) _direction "Forward")
        (switch Utilities|FlowControl|Switch|SwitchonENUM_NextOrPreviousLevel (Variables|Default|GetNextOrPreviousLevel)
          (:NewEnumerator0
            (Default|GotoNextLevel _nextlevel))
          (:NewEnumerator1
            (Default|GotoPreviousLevel _nextlevel)))))))

(event Custom|ResetReferences
  (Components|Timeline|SetPlayRate (Variables|Default|GetTl_TargetLerp) 3.0)
  (Utilities|FlowControl|Sequence
    (:then_0
      (bind _outactors (Actor|GetAllActorsOfClass "/Script/Engine.CameraActor"))
      (for _array_element _outactors
        (for _array_element_2 (Variables|/Script/Engine.Actor|GetTags _array_element)
          (if (Utilities|Name|Equal(Name) _array_element_2 "MainCamera")
            (Variables|Default|SetCamera _array_element)
            (Variables|CameraRotation|SetCameraRoot (Actor|GetAttachParentActor _array_element))
            (CallFunction|ReverseCamera)))))
    (:then_1
      (bind _outactors_2 (Actor|GetAllActorsOfClass "/Script/Engine.Actor"))
      (for _array_element_3 _outactors_2
        (if (Actor|ActorHasTag _array_element_3 "ReferenceRotation")
          (Variables|Default|SetReferenceRotation _array_element_3)
          (elif (Actor|ActorHasTag _array_element_3 "Lol")
            (Variables|Default|SetLol _array_element_3)))))
    (:then_2
      (bind _outactors_3 (Actor|GetAllActorsOfClass "/Game/Blueprints/NextLevel.NextLevel_C"))
      (Variables|Default|SetNextLevel (Utilities|Array|Get(acopy) _outactors_3)))
    (:then_3
      (bind _returnvalue (Actor|GetActorOfClass "/Script/Engine.PostProcessVolume"))
      (bind _output_get (Variables|Default|SetPostVolume _returnvalue))
      (Variables|/Script/Engine.PostProcessVolume|SetbEnabled _output_get true)
      (Audio|PlaySound2D "/Game/Sound/Music/Cues/Music.Music" 1.0 1.0 0.0 0 0))
    (:then_4
      ;[1 1 1] Set black screen
      (Utilities|Struct|SetmembersinPostProcessSettings (Variables|/Script/Engine.PostProcessVolume|GetSettings (Variables|Default|GetPostVolume)) (Math|Vector4|MakeVector4 0.0 0.0 0.0 0.0))
      ;[1 1 1] Set DOF to 1/10 of distance from camera to camera root, and camera correction for FOV
      (Utilities|Struct|SetmembersinPostProcessSettings (Variables|/Script/Engine.PostProcessVolume|GetSettings (Variables|Default|GetPostVolume)) (* (/ (Math|Vector|Distance(Vector) (Transformation|GetWorldLocation (Variables|/Script/Engine.CameraActor|GetCameraComponent (Variables|Default|GetCamera))) (Transformation|GetActorLocation (Variables|CameraRotation|GetCameraRoot))) 1e+01) (Math|Float|MapRangeUnclamped (Variables|/Script/Engine.CameraComponent|GetFieldOfView (Variables|/Script/Engine.CameraActor|GetCameraComponent (Variables|Default|GetCamera))) 4e+01 1.3e+02 3.0 0.3))))))

(event Custom|GoToNextLevel
  (Variables|Default|SetNextOrPreviousLevel "NewEnumerator0")
  (CallFunction|TriggerCompleteCamera))

(event Custom|CancelNextLevelTimer
  (Utilities|Time|PauseTimerbyHandle (Variables|Default|GetNextLevelTimer)))

(event Custom|GoToPreviousLevel
  (Variables|Default|SetNextOrPreviousLevel "NewEnumerator1")
  (CallFunction|TriggerCompleteCamera))

(event EventTick
  (params (DeltaSeconds :type Float%20%28single-precision%29))
  (bind _returnvalue (Game|GetPlayerCameraManager 0))
  (bind _returnvalue_2 (Camera|GetCameraLocation _returnvalue))
  (Utilities|FlowControl|Sequence
    (:then_0
      (Utilities|FlowControl|Sequence
        (:then_0
          (if (Variables|Default|GetSolved)
            (Variables|CameraRotation|SetCameraRotationTarget (+ (* (Utilities|Time|GetWorldDeltaSeconds) -1e+01) (Variables|CameraRotation|GetCameraRotationTarget)))
            (else
              (Utilities|FlowControl|Sequence
                (:then_0
                  (if (Variables|CameraRotation|GetRotate)
                    (Variables|CameraRotation|SetCameraRotationTarget (+ (* (Class|Actor|GetInputAxisKeyValue) 1e+01) (Variables|CameraRotation|GetCameraRotationTarget)))))
                (:then_1
                  (if (Variables|CameraRotation|GetRotate)
                    (Variables|CameraRotation|SetCameraRotationPitchTarget (Math|Float|Clamp(Float) (+ (* (Class|Actor|GetInputAxisKeyValue) 1e+01) (Variables|CameraRotation|GetCameraRotationPitchTarget)) -6e+01 2e+01))))))))
        (:then_2
          (bind _output_get (Variables|CameraRotation|SetCameraRotationYaw (Math|Interpolation|FInterpTo (Variables|CameraRotation|GetCameraRotationYaw) (Variables|CameraRotation|GetCameraRotationTarget) (Utilities|Time|GetWorldDeltaSeconds) 2.0)))
          (bind _output_get_2 (Variables|CameraRotation|SetCameraRotationPitch (Math|Interpolation|FInterpTo (Variables|CameraRotation|GetCameraRotationPitch) (Variables|CameraRotation|GetCameraRotationPitchTarget) (Utilities|Time|GetWorldDeltaSeconds) 2.0)))
          (Transformation|SetActorRotation (Variables|CameraRotation|GetCameraRoot) (Math|Rotator|MakeRotator 0.0 _output_get_2 _output_get)))))
    (:then_1
      (if (not (Variables|Default|GetSolved))
        (Utilities|FlowControl|Sequence
          (:then_1
            (if (Variables|CameraRotation|GetRotate)
              _
              (else
                _))
            ;[1 1 1] Detecting what mouse overlaps
            (bind _returnvalue_3 (Class|WidgetLayoutLibrary|GetMousePositiononPlatform))
            (Utilities|FlowControl|Sequence
              (:then_0
                (bind _outhit (Collision|LineTraceForObjects _returnvalue_2 (+ _returnvalue_2 (* (.WorldDirection (Class|GameplayStatics|DeprojectScreentoWorld (Game|GetPlayerController 0) (Math|Vector2D|MakeVector2D (.x (.PixelPosition (Class|SlateBlueprintLibrary|AbsolutetoViewport (Math|Vector2D|MakeVector2D (.x _returnvalue_3) (.y _returnvalue_3))))) (.y (.PixelPosition (Class|SlateBlueprintLibrary|AbsolutetoViewport (Math|Vector2D|MakeVector2D (.x _returnvalue_3) (.y _returnvalue_3)))))))) 5e+03)) (Utilities|Array|MakeArray "ObjectTypeQuery1") false 0 "None"))
                (Variables|Default|SetPhysicsHandleWorldLocation (.location _outhit)))
              (:then_1
                (bind (_outhit_2 _returnvalue_4) (Collision|LineTraceByChannel _returnvalue_2 (+ _returnvalue_2 (* (.WorldDirection (Class|GameplayStatics|DeprojectScreentoWorld (Game|GetPlayerController 0) (Math|Vector2D|MakeVector2D (.x (.PixelPosition (Class|SlateBlueprintLibrary|AbsolutetoViewport (Math|Vector2D|MakeVector2D (.x _returnvalue_3) (.y _returnvalue_3))))) (.y (.PixelPosition (Class|SlateBlueprintLibrary|AbsolutetoViewport (Math|Vector2D|MakeVector2D (.x _returnvalue_3) (.y _returnvalue_3)))))))) 5e+03)) "TraceTypeQuery1" false 0 "None"))
                (if _returnvalue_4
                  (Utilities|IsValid (Actor|GetComponentbyClass (.hitactor _outhit_2) "/Game/Blueprints/DragComponent.DragComponent_C")
                    (:Is%20Valid
                      (CallFunction|SetOverlap (.hitactor _outhit_2)))
                    (:Is%20Not%20Valid
                      (CallFunction|SetOverlap :!label _label)))
                  (else
                    (goto _label))))))
          (:then_2
            (Physics|Components|PhysicsHandle|SetTargetLocation (Variables|Default|GetPhysicsHandle) (Math|Vector|MakeVector (Math|Float|Clamp(Float) (.x (Math|Vector|SelectVector (Variables|Default|GetTargetLerp) (+ (Variables|Default|GetPhysicsHandleWorldLocation) (Variables|Default|GetPhysicsOffset) (Math|Vector|MakeVector 0.0 0.0 (Variables|Default|GetLift))) (Variables|Default|GetTargetLerpActive))) -6e+02 7e+02) (Math|Float|Clamp(Float) (.y (Math|Vector|SelectVector (Variables|Default|GetTargetLerp) (+ (Variables|Default|GetPhysicsHandleWorldLocation) (Variables|Default|GetPhysicsOffset) (Math|Vector|MakeVector 0.0 0.0 (Variables|Default|GetLift))) (Variables|Default|GetTargetLerpActive))) -8e+02 5e+02) (Math|Float|Clamp(Float) (.z (Math|Vector|SelectVector (Variables|Default|GetTargetLerp) (+ (Variables|Default|GetPhysicsHandleWorldLocation) (Variables|Default|GetPhysicsOffset) (Math|Vector|MakeVector 0.0 0.0 (Variables|Default|GetLift))) (Variables|Default|GetTargetLerpActive))) 0.0 4e+02)))))))))

(event EventBeginPlay
  (Components|Timeline|SetPlayRate (Variables|Default|GetTl_TargetLerp) 3.0)
  (Utilities|FlowControl|Sequence
    (:then_0
      (bind _outactors (Actor|GetAllActorsOfClass "/Script/Engine.CameraActor"))
      (for _array_element _outactors
        (for _array_element_2 (Variables|/Script/Engine.Actor|GetTags _array_element)
          (if (Utilities|Name|Equal(Name) _array_element_2 "MainCamera")
            (Variables|Default|SetCamera _array_element)
            (Variables|CameraRotation|SetCameraRoot (Actor|GetAttachParentActor _array_element))
            (CallFunction|ReverseCamera)))))
    (:then_1
      (bind _outactors_2 (Actor|GetAllActorsOfClass "/Script/Engine.Actor"))
      (for _array_element_3 _outactors_2
        (if (Actor|ActorHasTag _array_element_3 "ReferenceRotation")
          (Variables|Default|SetReferenceRotation _array_element_3)
          (elif (Actor|ActorHasTag _array_element_3 "Lol")
            (Variables|Default|SetLol _array_element_3)))))
    (:then_2
      (bind _outactors_3 (Actor|GetAllActorsOfClass "/Game/Blueprints/NextLevel.NextLevel_C"))
      (Variables|Default|SetNextLevel (Utilities|Array|Get(acopy) _outactors_3)))
    (:then_3
      (bind _returnvalue (Actor|GetActorOfClass "/Script/Engine.PostProcessVolume"))
      (bind _output_get (Variables|Default|SetPostVolume _returnvalue))
      (Variables|/Script/Engine.PostProcessVolume|SetbEnabled _output_get true)
      (Audio|PlaySound2D "/Game/Sound/Music/Cues/Music.Music" 1.0 1.0 0.0 0 0))
    (:then_4
      ;[1 1 1] Set black screen
      (Utilities|Struct|SetmembersinPostProcessSettings (Variables|/Script/Engine.PostProcessVolume|GetSettings (Variables|Default|GetPostVolume)) (Math|Vector4|MakeVector4 0.0 0.0 0.0 0.0))
      ;[1 1 1] Set DOF to 1/10 of distance from camera to camera root, and camera correction for FOV
      (Utilities|Struct|SetmembersinPostProcessSettings (Variables|/Script/Engine.PostProcessVolume|GetSettings (Variables|Default|GetPostVolume)) (* (/ (Math|Vector|Distance(Vector) (Transformation|GetWorldLocation (Variables|/Script/Engine.CameraActor|GetCameraComponent (Variables|Default|GetCamera))) (Transformation|GetActorLocation (Variables|CameraRotation|GetCameraRoot))) 1e+01) (Math|Float|MapRangeUnclamped (Variables|/Script/Engine.CameraComponent|GetFieldOfView (Variables|/Script/Engine.CameraActor|GetCameraComponent (Variables|Default|GetCamera))) 4e+01 1.3e+02 3.0 0.3))))))

(event Input|ActionEvents|InputActionPauseMenu
  (params (Key :type Key%20Structure :default "None"))
  (bind _hudmanager (Variables|Default|GetHUDManager))
  (:Pressed
    (Utilities|FlowControl|FlipFlop
      (:A
        (Default|AddHUDPause _hudmanager))
      (:B
        (Default|RemoveHUDPause _hudmanager)))))

(event Input|MouseEvents|LeftMouseButton
  (params (Key :type Key%20Structure :default "None"))
  (bind _inputenabled (CallFunction|IsInputEnabled))
  (:Pressed
    (if _inputenabled
      (bind _overlap_actor (Variables|Default|GetOverlap%20Actor)
        (:then
          (CallFunction|SetHeld _overlap_actor))
        (:else))))
  (:Released
    (if _inputenabled
      (CallFunction|SetHeld))))

(event Input|MouseEvents|RightMouseButton
  (params (Key :type Key%20Structure :default "None"))
  (bind _inputenabled (CallFunction|IsInputEnabled))
  (:Pressed
    (if _inputenabled
      (Variables|CameraRotation|SetRotate true)))
  (:Released
    (if _inputenabled
      (Variables|CameraRotation|SetRotate false))))

(event Input|MouseEvents|MouseWheelDown
  (params (Key :type Key%20Structure :default "None"))
  (:Pressed
    (Variables|Default|SetLift (Math|Float|Clamp(Float) (- (Variables|Default|GetLift) 1e+01) -3e+02 3e+02))))

(event Input|MouseEvents|MouseWheelUp
  (params (Key :type Key%20Structure :default "None"))
  (:Pressed
    (Variables|Default|SetLift (Math|Float|Clamp(Float) (+ (Variables|Default|GetLift) 1e+01) -3e+02 3e+02))))

(event Input|KeyboardEvents|W
  (params (Key :type Key%20Structure :default "None"))
  (:Pressed
    (Timeline|TL_Loop Play
      (:Update
        (Variables|Default|GetHeld%20Actor
          (:then
            (CallFunction|Update (Math|Rotator|MakeRotator 0.0 (* (Utilities|Time|GetWorldDeltaSeconds) -1e+02) 0.0)))
          (:else)))))
  (:Released
    (Timeline|TL_Loop Stop)))

(event Input|KeyboardEvents|S
  (params (Key :type Key%20Structure :default "None"))
  (:Pressed
    (Timeline|Timeline_0 Play
      (:Update
        (Variables|Default|GetHeld%20Actor
          (:then
            (CallFunction|Update (Math|Rotator|MakeRotator 0.0 (* (Utilities|Time|GetWorldDeltaSeconds) 1e+02) 0.0)))
          (:else)))))
  (:Released
    (Timeline|Timeline_0 Stop)))

(event Input|KeyboardEvents|A
  (params (Key :type Key%20Structure :default "None"))
  (:Pressed
    (Timeline|Timeline_1 Play
      (:Update
        (Variables|Default|GetHeld%20Actor
          (:then
            (CallFunction|Update (Math|Rotator|MakeRotator 0.0 0.0 (* (Utilities|Time|GetWorldDeltaSeconds) 1e+02))))
          (:else)))))
  (:Released
    (Timeline|Timeline_1 Stop)))

(event Input|KeyboardEvents|D
  (params (Key :type Key%20Structure :default "None"))
  (:Pressed
    (Timeline|Timeline_2 Play
      (:Update
        (Variables|Default|GetHeld%20Actor
          (:then
            (CallFunction|Update (Math|Rotator|MakeRotator 0.0 0.0 (* (Utilities|Time|GetWorldDeltaSeconds) -1e+02))))
          (:else)))))
  (:Released
    (Timeline|Timeline_2 Stop)))

(fn ConstructionScript)

(fn IsInputEnabled
  (return (not (Variables|/Game/Blueprints/HUDManager.HUDManager_C|GetBlockInput (Variables|Default|GetHUDManager)))))