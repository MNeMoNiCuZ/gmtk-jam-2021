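; ConnectorComponent is a scene component that marks a connection point, apparently for puzzle pieces, with a radius and solved state.
; When debug drawing is on, Tick draws a sphere that is green if solved or always solved, red otherwise.
; BeginPlay caches all BP_Piece_Base actors, used only by an unreachable distance debug print.
; The file only reads the solved state and never sets it.
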(event EventBeginPlay
  (bind _outactors (Actor|GetAllActorsOfClass "/Game/Pieces/BP_Piece_Base.BP_Piece_Base_C"))
  (Variables|Default|SetPieceActors _outactors))

(event EventTick
  (params (DeltaSeconds :type Float%20%28single-precision%29))
  (if (Variables|Default|GetDebug%20Draw)
    (Rendering|Debug|DrawDebugSphere (Transformation|GetWorldLocation self) (Variables|Default|GetRadius) 12 (Math|Color|SelectColor "(R=0.095340,G=1.000000,B=0.035684,A=1.000000)" "(R=1.000000,G=0.000000,B=0.000000,A=1.000000)" (or (Variables|Default|GetSolved) (Variables|Default|GetAlwaysSolved))) 0.0 1.0)))