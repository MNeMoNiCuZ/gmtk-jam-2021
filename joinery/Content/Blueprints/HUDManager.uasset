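; HUD manager Blueprint that shows and hides the puzzle game's controls, level-complete and pause screens.
; Each screen has an Add event that creates the widget for the PuzzlePlayerController, stores it and adds it to the viewport.
; Matching Remove events take the widget off screen and clear the reference.
; The pause events also toggle a BlockInput flag, setting it while the pause menu is up.
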(event Custom|AddHUDControls
  (bind _aspuzzle_player_controller (Utilities|Casting|CastToPuzzlePlayerController (Game|GetPlayerController 0)))
  (bind _returnvalue (UserInterface|CreateWidget "/Game/UI/HUD_Controls.HUD_Controls_C" _aspuzzle_player_controller))
  (bind _output_get (Variables|Default|SetHUD_Controls _returnvalue))
  (UserInterface|Viewport|AddtoViewport _output_get 0))

(event Custom|RemoveHUDControls
  (Utilities|Casting|CastToPuzzlePlayerController (Game|GetPlayerController 0))
  (Widget|RemovefromParent (Variables|Default|GetHUD_Controls))
  (Variables|Default|SetHUD_Controls 0))

(event Custom|AddHUDLevelComplete
  (bind _aspuzzle_player_controller (Utilities|Casting|CastToPuzzlePlayerController (Game|GetPlayerController 0)))
  (bind _returnvalue (UserInterface|CreateWidget "/Game/UI/HUD_LevelComplete.HUD_LevelComplete_C" _aspuzzle_player_controller))
  (bind _output_get (Variables|Default|SetHUD_LevelComplete _returnvalue))
  (UserInterface|Viewport|AddtoViewport _output_get 0))

(event Custom|RemoveHUDLevelComplete
  (Utilities|Casting|CastToPuzzlePlayerController (Game|GetPlayerController 0))
  (Widget|RemovefromParent (Variables|Default|GetHUD_LevelComplete))
  (Variables|Default|SetHUD_LevelComplete 0))

(event Custom|AddHUDPause
  (bind _aspuzzle_player_controller (Utilities|Casting|CastToPuzzlePlayerController (Game|GetPlayerController 0)))
  (bind _returnvalue (UserInterface|CreateWidget "/Game/UI/HUD_Pause.HUD_Pause_C" _aspuzzle_player_controller))
  (bind _output_get (Variables|Default|SetHUD_PauseMenu _returnvalue))
  (UserInterface|Viewport|AddtoViewport _output_get 0)
  (Variables|Default|SetBlockInput true))

(event Custom|RemoveHUDPause
  (Utilities|Casting|CastToPuzzlePlayerController (Game|GetPlayerController 0))
  (Widget|RemovefromParent (Variables|Default|GetHUD_PauseMenu))
  (Variables|Default|SetHUD_PauseMenu 0)
  (Variables|Default|SetBlockInput false))