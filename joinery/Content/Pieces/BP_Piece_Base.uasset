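; Base puzzle piece that reports whether all its connectors are matched with those of other pieces.
; Each tick it resets its connectors, distance-tests them against every other piece's, recolors editor-style billboard icons red/green, then calls solved or not solved.
; Always-solved connectors skip the requirement.
; Slide volume follows velocity while hits are recent; impacts play throttled light or heavy wood sounds by impulse.
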(event Custom|SetSlideVolume
  (Audio|Components|Audio|SetVolumeMultiplier (Variables|Default|GetSlideAudio) (Math|Float|SelectFloat (Math|Float|MapRangeClamped (Math|Vector|VectorLength (Transformation|GetVelocity)) 5e+01 1e+03 0.0 1.0) 0.0 (<= (Variables|Default|GetTimeSinceLastHit) 0.2)) :!class /Script/Engine.AudioComponent))

(event Collision|EventHit
  (params (MyComp :type Primitive%20Component%20Object%20Reference) (Other :type Actor%20Object%20Reference) (OtherComp :type Primitive%20Component%20Object%20Reference) (bSelfMoved :type Boolean) (HitLocation :type Vector :default "0, 0, 0") (HitNormal :type Vector :default "0, 0, 0") (NormalImpulse :type Vector :default "0, 0, 0") (Hit :type Hit%20Result%20Structure%20%28by%20ref%29))
  (bind _returnvalue (Transformation|GetVelocity))
  (bind _returnvalue_2 (Math|Vector|VectorLength _returnvalue))
  (bind _returnvalue_3 (Math|Float|MapRangeClamped _returnvalue_2 5e+01 1e+03 0.0 0.1))
  (Variables|Default|SetTimeSinceLastHit 0.0)
  ;[1 1 1] Impact Sounds
  (Utilities|FlowControl|DoOnce false :!label _label
    (:Completed
      (if (>= (Math|Vector|VectorLength NormalImpulse) 1.5e+04)
        (Audio|PlaySoundatLocation "/Game/Sound/Impacts/Cues/WoodImpactHeavy.WoodImpactHeavy" HitLocation "0, 0, 0" _returnvalue_3 1.0 0.0 0 0 0)
        (else
          (Audio|PlaySoundatLocation "/Game/Sound/Impacts/Cues/WoodImpactLight.WoodImpactLight" HitLocation "0, 0, 0" _returnvalue_3 1.0 0.0 0 0 0)))
      (Utilities|FlowControl|Delay 0.25)
      (goto _label Reset))))

(event EventTick
  (params (DeltaSeconds :type Float%20%28single-precision%29))
  (Variables|Default|SetTimeSinceLastHit (+ DeltaSeconds (Variables|Default|GetTimeSinceLastHit)))
  (CallFunction|SetSlideVolume)
  ;[1 1 1] Reset
  (for _array_element (Variables|Default|GetSelfConnectors)
    (Variables|/Game/Blueprints/ConnectorComponent.ConnectorComponent_C|SetSolved _array_element false))
  (Rendering|Components|Sprite|SetSprite (Variables|Default|GetSelfConnectorIcons) "/Game/Textures/TEX_ConnectorIcon_Red.TEX_ConnectorIcon_Red")
  (for _array_element_2 (Variables|Default|GetOtherPieceActors)
    (bind _output_get (Variables|Default|SetCacheOtherConnectors (Actor|GetComponentsByClass _array_element_2 "/Game/Blueprints/ConnectorComponent.ConnectorComponent_C")))
    (bind _array_element_3 (Utilities|Array|ForEachLoopwithBreak _output_get)
      (:LoopBody
        (bind _output_get_2 (Variables|Default|SetCacheSpecificConnector _array_element_3))
        (Variables|Default|SetCachedDistanceTolerance (Variables|/Game/Blueprints/ConnectorComponent.ConnectorComponent_C|GetRadius _output_get_2))
        (bind (_array_element_4 _array_index) (Utilities|Array|ForEachLoopwithBreak (Variables|Default|GetSelfConnectors))
          (:LoopBody
            (if (<= (Math|Vector|Distance(Vector) (Transformation|GetWorldLocation (Variables|Default|GetCacheSpecificConnector)) (Transformation|GetWorldLocation _array_element_4)) (Variables|/Game/Blueprints/ConnectorComponent.ConnectorComponent_C|GetRadius _array_element_4))
              (Variables|/Game/Blueprints/ConnectorComponent.ConnectorComponent_C|SetSolved _array_element_4 true)
              (Rendering|Components|Sprite|SetSprite (Utilities|Array|Get(acopy) (Variables|Default|GetSelfConnectorIcons) _array_index) "/Game/Textures/TEX_ConnectorIcon_Green.TEX_ConnectorIcon_Green")))))))
  ;[1 1 1] Check if this piece is solved
  (Utilities|FlowControl|Sequence
    (:then_0
      (Variables|Default|SetUnsolved false)
      (bind _array_element_5 (Utilities|Array|ForEachLoopwithBreak (Variables|Default|GetSelfConnectors) :!label _label)
        (:LoopBody
          (if (not (or (Variables|/Game/Blueprints/ConnectorComponent.ConnectorComponent_C|GetSolved _array_element_5) (Variables|/Game/Blueprints/ConnectorComponent.ConnectorComponent_C|GetAlwaysSolved _array_element_5)))
            (Variables|Default|SetUnsolved true)
            (goto _label Break)))
        (:Completed
          (if (Variables|Default|GetUnsolved)
            (Default|CallPieceNotSolved)
            (else
              (Default|CallPieceSolved))))))))

(event EventBeginPlay
  (bind _outactors (Actor|GetAllActorsOfClass "BP_Piece_Base_C"))
  (bind _output_get (Variables|Default|SetOtherPieceActors _outactors))
  (Utilities|Array|RemoveItem _output_get self))

(fn ConstructionScript
  (bind _output_get (Variables|Default|SetSelfConnectors (Actor|GetComponentsByClass "/Game/Blueprints/ConnectorComponent.ConnectorComponent_C")))
  (for _array_element _output_get
    (if (Variables|/Game/Blueprints/ConnectorComponent.ConnectorComponent_C|GetAlwaysSolved _array_element) ; Doesn't work, never shows true
      (bind _returnvalue (AddComponent|AddBillboardComponent false (Math|Transform|MakeTransform (Variables|/Script/Engine.SceneComponent|GetRelativeLocation _array_element) "0, 0, 0" (Math|Conversions|ToVector(Float) (Math|Float|MapRangeClamped (Variables|/Game/Blueprints/ConnectorComponent.ConnectorComponent_C|GetRadiusVisual _array_element) 0.0 1e+02 0.0 1.0)))))
      (Development|SetHiddeninGame _returnvalue true false)
      (Utilities|Array|Add (Variables|Default|GetSelfConnectorIcons) _returnvalue)
      (else
        (bind _returnvalue_2 (AddComponent|AddBillboardComponent false (Math|Transform|MakeTransform (Variables|/Script/Engine.SceneComponent|GetRelativeLocation _array_element) "0, 0, 0" (Math|Conversions|ToVector(Float) (Math|Float|MapRangeClamped (Variables|/Game/Blueprints/ConnectorComponent.ConnectorComponent_C|GetRadiusVisual _array_element) 0.0 1e+02 0.0 1.0)))))
        (Development|SetHiddeninGame _returnvalue_2 true false)
        (Utilities|Array|Add (Variables|Default|GetSelfConnectorIcons) _returnvalue_2)))))

(fn IsSelfHeld
  (bind _aspuzzle_player_character (Utilities|Casting|CastToPuzzlePlayerCharacter (Game|GetPlayerCharacter 0)))
  (return (== (Variables|/Game/Blueprints/PuzzlePlayerCharacter.PuzzlePlayerCharacter_C|GetHeld%20Actor _aspuzzle_player_character) self)))